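; Base game mode that spawns players at the level's PlayerStarts and can reset the round.
; On BeginPlay, GameStart caches every PlayerStart, spawns a BasePlayerBP at each and stores it in Players.
; Player controller 0 possesses each pawn in turn, so it ends on the last one spawned.
; Reset destroys all BaseProjectileBP actors and moves each player back to the start with the matching index.
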(event Custom|GameStart
  ;[1 1 1] Spawn and poses players
  (bind _outactors (Actor|GetAllActorsOfClass "/Script/Engine.PlayerStart"))
  (bind _output_get (Variables|Default|SetPlayerStarts _outactors))
  (for _array_element _output_get
    (bind _returnvalue (Game|SpawnActorfromClass "/Game/Blueprints/BasePlayerBP.BasePlayerBP_C" (Transformation|GetActorTransform _array_element) "Undefined" _array_element 0))
    (Utilities|Array|Add (Variables|Default|GetPlayers) _returnvalue)
    (Pawn|Possess (Game|GetPlayerController 0) _returnvalue)))

(event Custom|Reset
  ;[1 1 1] Reset position and destroy all bullets
  (bind _outactors (Actor|GetAllActorsOfClass "/Game/Blueprints/BaseProjectileBP.BaseProjectileBP_C"))
  (for _array_element _outactors
    (Actor|DestroyActor _array_element))
  (for (_array_element_2 _array_index) (Variables|Default|GetPlayers)
    (Transformation|SetActorTransform _array_element_2 (Transformation|GetActorTransform (Utilities|Array|Get(acopy) (Variables|Default|GetPlayerStarts) _array_index)))))

(event EventBeginPlay
  (CallFunction|GameStart))

(event EventTick
  (params (DeltaSeconds :type Float%20%28single-precision%29)))

(fn ConstructionScript)