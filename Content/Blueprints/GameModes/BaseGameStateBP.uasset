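; Base game state Blueprint that tracks the list of players and a score for each.
; GetAllPlayers gathers every BasePlayerBP actor into Players and adds each to the Score map at zero.
; AddScore has the target add one point to itself, stores the returned value in the map, then fires the ScoreChange dispatcher with the new score and target.
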(event Custom|AddScore
  (params (Target :type Base%20Player%20BP%20Object%20Reference))
  (bind _score (Variables|Default|GetScore))
  (bind _returnvalue (Class|BasePlayer|AddScore Target 1))
  (Utilities|Map|Remove _score Target)
  (Utilities|Map|Add _score Target _returnvalue)
  (Default|CallScoreChange _returnvalue Target))

(event Custom|GetAllPlayers
  (bind _outactors (Actor|GetAllActorsOfClass "/Game/Blueprints/BasePlayerBP.BasePlayerBP_C"))
  (bind _output_get (Variables|Default|SetPlayers _outactors))
  (for _array_element _output_get
    (Utilities|Map|Add (Variables|Default|GetScore) _array_element 0)))

(event EventBeginPlay)

(event EventTick
  (params (DeltaSeconds :type Float%20%28single-precision%29)))

(fn ConstructionScript)