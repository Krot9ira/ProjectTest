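; BasePlayerBP is the player Blueprint, which sets up the score UI and registers a player with the AI on BeginPlay.
; It creates a Score_WBP widget for player controller 0 and adds it to the viewport.
; It then writes the first BasePlayerBP found into the blackboard of only the second BaseAIController found, if that blackboard is valid.
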(event EventBeginPlay
  (bind _returnvalue (UserInterface|CreateWidget "/Game/Blueprints/Widgets/Score_WBP.Score_WBP_C" (Game|GetPlayerController 0)))
  (UserInterface|Viewport|AddtoViewport _returnvalue 0)
  (bind _outactors (Actor|GetAllActorsOfClass "/Script/ProjectTest.BaseAIController"))
  (bind _outactors_2 (Actor|GetAllActorsOfClass "BasePlayerBP_C"))
  (Utilities|IsValid (AI|GetBlackboard (Utilities|Array|Get(acopy) _outactors 1))
    (:Is%20Valid
      (AI|Components|Blackboard|SetValueasObject (AI|GetBlackboard (Utilities|Array|Get(acopy) _outactors 1)) (Variables|Default|GetKey%20Name) (Utilities|Array|Get(acopy) _outactors_2)))))

(fn ConstructionScript)