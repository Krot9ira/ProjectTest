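; Base projectile Blueprint that scores a point for its shooter and resets the game when it hits another player.
; On sphere overlap, it ignores anything that is not a BasePlayerBP, as well as its own Instigator.
; A valid hit passes the Instigator to AddScore on the game state, then calls Reset on the game mode.
; The graph holds no movement, damage or destroy logic.
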(event OnComponentBeginOverlap(SphereCollision)
  (params (OverlappedComponent :type Primitive%20Component%20Object%20Reference) (OtherActor :type Actor%20Object%20Reference) (OtherComp :type Primitive%20Component%20Object%20Reference) (OtherBodyIndex :type Integer) (bFromSweep :type Boolean) (SweepResult :type Hit%20Result%20Structure%20%28by%20ref%29))
  (bind _returnvalue (Game|GetInstigator))
  (Utilities|Casting|CastToBasePlayerBP OtherActor)
  (if (!= OtherActor _returnvalue)
    (bind _asbase_game_state_bp (Utilities|Casting|CastToBaseGameStateBP (Game|GetGameState)))
    (bind _asbase_player_bp (Utilities|Casting|CastToBasePlayerBP _returnvalue))
    (Default|AddScore _asbase_game_state_bp _asbase_player_bp)
    (bind _asbase_game_mode_bp (Utilities|Casting|CastToBaseGameModeBP (Game|GetGameMode)))
    (Default|Reset _asbase_game_mode_bp)))

(event EventBeginPlay)

(event Collision|EventActorBeginOverlap
  (params (OtherActor :type Actor%20Object%20Reference)))

(event EventTick
  (params (DeltaSeconds :type Float%20%28single-precision%29)))

(fn ConstructionScript)